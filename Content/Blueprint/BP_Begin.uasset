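; BP_Begin is an actor that sets up the opening state of a level, playing an intro sequence while the player is held in place.
; On BeginPlay it caches the BP_Player found in the world, switches input to UI only, disables that player's movement and shows the mouse cursor.
; It plays its referenced Level Sequence if valid, and contains no logic to restore movement or input afterward.
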(event `self.ReceiveBeginPlay`
  (`self.Setup Variables`)
  (`WidgetBlueprintLibrary.SetInputMode_UIOnlyEx` (`GameplayStatics.GetPlayerController` 0) null)
  (set `/Game/Blueprint/BP_Player.Can Move` false (`self.Player`))
  (`self.TriggerAnimation`)
  (set `PlayerController.bShowMouseCursor` true (`GameplayStatics.GetPlayerController` 0)))

(event `TriggerAnimation`
  (bind _levelsequence (`self.LevelSequence`))
  (`/Engine/EditorBlueprintResources/StandardMacros.IsValid` _levelsequence
    (:`Is Valid`
      (`MovieSceneSequencePlayer.Play` (`LevelSequenceActor.SequencePlayer` _levelsequence)))))

(event `Setup Variables`
  (bind _returnvalue (`GameplayStatics.GetActorOfClass` "/Game/Blueprint/BP_Player.BP_Player_C"))
  (set `self.Player` _returnvalue))

(fn `UserConstructionScript`)