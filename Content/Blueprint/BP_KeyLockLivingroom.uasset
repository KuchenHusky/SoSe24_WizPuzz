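; Living room key lock that plays a level sequence, presumably the door opening, when the matching key is brought to it.
; Its box collider detects actors tagged Key, casts them to BP_Pickup_Child_Key and compares the key's name to WantedKey.
; A match plays a sound, destroys the pickup and reveals the lock's own key component.
; The opened flag blocking further triggers is set only when a valid sequence plays.
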(event `Setup Variables`)

(event `self.Box_Collider.OnComponentBeginOverlap`
  (params (OverlappedComponent :type "PrimitiveComponent Object Reference") (OtherActor :type "Actor Object Reference") (OtherComp :type "PrimitiveComponent Object Reference") (OtherBodyIndex :type Integer) (bFromSweep :type Boolean) (SweepResult :type "HitResult Structure (by ref)"))
  (bind _returnvalue (`self.ActorHasTag` OtherActor "Key"))
  (bind _level_sequence_to_play (`self.Level Sequence to Play`))
  (if (`self.Door Is Opend`)
    _
    (elif _returnvalue
      (`KismetSystemLibrary.PrintString` (`KismetStringLibrary.Conv_BoolToString` _returnvalue))
      (bind _asbp_pickup_child_key (cast `/Game/Blueprint/BP_Pickup/BP_Pickup_Child_Key` OtherActor))
      (bind _output_get (set `self.Current Key` _asbp_pickup_child_key))
      (bind _returnvalue_2 (`KismetStringLibrary.EqualEqual_StrStr` (`self.Wanted Key`) (`/Game/Blueprint/BP_Pickup/BP_Pickup_Child_Key.KeyName` _output_get)))
      (`KismetSystemLibrary.PrintString` (`KismetStringLibrary.Conv_BoolToString` _returnvalue_2))
      (if _returnvalue_2
        (`GameplayStatics.PlaySound2D` "/Game/Sounds/DoneSound/DoneSound.DoneSound" 1.0 1.0 0.0 null null)
        (`self.K2_DestroyActor` (`self.Current Key`))
        (`SceneComponent.SetVisibility` (`self.Key_Livingroom`) true false)
        (`/Engine/EditorBlueprintResources/StandardMacros.IsValid` _level_sequence_to_play
          (:`Is Valid`
            (`MovieSceneSequencePlayer.Play` (`LevelSequenceActor.SequencePlayer` _level_sequence_to_play))
            (set `self.Door Is Opend` true)))))))

(fn `UserConstructionScript`)