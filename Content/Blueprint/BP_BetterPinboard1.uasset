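; Interactable pinboard pawn, built on keypad logic, where the player browses notes and opens post-it hints.
; Interact smoothly possesses the board, locks player movement, hides gameplay UI and adds a keypad input mapping context.
; Directional inputs move a highlight across a wrapping grid of button components, and confirm shows that index's hint widget.
; Back re-possesses the previous pawn; a separate event floor-traces to reposition it, while button animation is unwired.
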(event `SetButtonHighlighted`
  (params (Position :type Integer) (Highlight :type Boolean))
  ;[1 1 1] Set Button Highlight
  (`/Game/Blueprint/Components/BPC_KeypadButton.SetHighlight` (`|GetArrayItem` (`self.Button List`) Position) Highlight))

(event `self.SetHighlight`
  (params (On :type Boolean))
  ;[1 1 1] Set Highlight
  (`MeshComponent.SetOverlayMaterial` (`self.SM_Pinnwall`) (select `bool` On :`true` "/Game/Materials/Overlays/M_WaveyTexture.M_WaveyTexture" :!type "MaterialInterface Object Reference")))

(event `self.ReceivePossessed`
  (params (NewController :type "Controller Object Reference"))
  ;[1 1 1] Possedess
  (`EnhancedInputSubsystemInterface.AddMappingContext` (pcsubsystem `EnhancedInputLocalPlayerSubsystem` (`GameplayStatics.GetPlayerController` 0)) "/Game/Inputs/Keypad/IMC_Keypad.IMC_Keypad" 0 (struct)))

(event `self.ReceiveUnpossessed`
  (params (OldController :type "Controller Object Reference"))
  ;[1 1 1] Possedess
  (`EnhancedInputSubsystemInterface.RemoveMappingContext` (pcsubsystem `EnhancedInputLocalPlayerSubsystem` (`GameplayStatics.GetPlayerController` 0)) "/Game/Inputs/Keypad/IMC_Keypad.IMC_Keypad" (struct))
  (`Widget.SetVisibility` (`/Game/UI/WBP_GameUI.GameplayStack` (`/Game/Blueprint/GM_Basic.GameUI` (`/Game/Blueprint/BP_Player.Game Mode` (`self.Player`)))) "Visible"))

(event `self.Interact`
  (params (`Last Possess` :type "Pawn Object Reference"))
  ;[1 1 1] Interact
  (bind _output_get (set `self.Last Possess` `Last Possess`))
  (`|ExecutionSequence`
    (:`then_0`
      (`/Game/Blueprint/BP_MacroLibary.MySmoothPossess` self 0.5)
      (bind _output_get_2 (set `self.Current Button` 0))
      (`self.SetButtonHighlighted` _output_get_2 true))
    (:`then_1`
      (bind _asbp_player (cast `/Game/Blueprint/BP_Player` _output_get))
      (set `self.Player` _asbp_player)
      (set `/Game/Blueprint/BP_Player.Can Move` false _asbp_player)
      (set `self.Last Posses Capsile half height` (`CapsuleComponent.GetScaledCapsuleHalfHeight` (`Character.CapsuleComponent` _asbp_player)))
      (`Widget.SetVisibility` (`/Game/UI/WBP_GameUI.GameplayStack` (`/Game/Blueprint/GM_Basic.GameUI` (`/Game/Blueprint/BP_Player.Game Mode` _asbp_player))) "Hidden"))))

(event `Exit Keypad`
  ;[1 1 1] Exit Keypad
  (`self.SetButtonHighlighted` (`self.Current Button`))
  (`self.DisableInput` null)
  (`/Game/Blueprint/BP_MacroLibary.MySmoothPossess` (`self.Last Possess`) 0.5)
  (`self.EnableInput` null))

(event `AnimateButton`
  ;[1 1 1] AnimateButton
)

(event `Reposition Player`
  ;[1 1 1] Reposition Player
  (bind _outhit (`KismetSystemLibrary.LineTraceSingle` (+ (`SceneComponent.K2_GetComponentLocation` (`self.PlayerPos`)) (0.0 0.0 -250.0)) (0.0 0.0 0.0) "TraceTypeQuery1"))
  (`self.K2_SetActorLocationAndRotation` (`self.Last Possess`) (+ (`.Location` (`GameplayStatics.BreakHitResult` _outhit)) (`KismetMathLibrary.MakeVector` 0.0 0.0 (+ (`self.Last Posses Capsile half height`) 2.0))) (`SceneComponent.K2_GetComponentRotation` (`self.PlayerPos`)) false false))

(event `EnhancedInput|/Game/Inputs/IA_Back`
  (params (ActionValue :type Boolean) (ElapsedSeconds :type "Float (double-precision)") (TriggeredSeconds :type "Float (double-precision)") (InputAction :type "InputAction Object Reference" :default "/Game/Inputs/IA_Back.IA_Back"))
  ;[1 1 1] Back
  (:`Started`
    (`self.Exit Keypad`)))

(event `EnhancedInput|/Game/Inputs/Keypad/IA_Right`
  (params (ActionValue :type Boolean) (ElapsedSeconds :type "Float (double-precision)") (TriggeredSeconds :type "Float (double-precision)") (InputAction :type "InputAction Object Reference" :default "/Game/Inputs/Keypad/IA_Right.IA_Right"))
  ;[1 1 1] Right
  (:`Started`
    (`self.SetButtonHighlighted` (`self.Current Button`))
    (bind _result (`/Engine/EditorBlueprintResources/StandardMacros.IncrementInt` (`self.Current Button`))
      (:`  `
        (if (not (< _result (`KismetArrayLibrary.Array_Length` (`self.Button List`))))
          (set `self.Current Button` 0))
        (`self.SetButtonHighlighted` (`self.Current Button`) true)))))

(event `EnhancedInput|/Game/Inputs/Keypad/IA_Left`
  (params (ActionValue :type Boolean) (ElapsedSeconds :type "Float (double-precision)") (TriggeredSeconds :type "Float (double-precision)") (InputAction :type "InputAction Object Reference" :default "/Game/Inputs/Keypad/IA_Left.IA_Left"))
  ;[1 1 1] Left
  (:`Started`
    (`self.SetButtonHighlighted` (`self.Current Button`))
    (bind _result (`/Engine/EditorBlueprintResources/StandardMacros.DecrementInt` (`self.Current Button`))
      (:`  `
        (if (not (> _result -1))
          (bind _result_2 (`/Engine/EditorBlueprintResources/StandardMacros.DecrementInt` (`KismetArrayLibrary.Array_Length` (`self.Button List`)))
            (:`  `
              (set `self.Current Button` _result_2))))
        (`self.SetButtonHighlighted` (`self.Current Button`) true)))))

(event `EnhancedInput|/Game/Inputs/Keypad/IA_Down`
  (params (ActionValue :type Boolean) (ElapsedSeconds :type "Float (double-precision)") (TriggeredSeconds :type "Float (double-precision)") (InputAction :type "InputAction Object Reference" :default "/Game/Inputs/Keypad/IA_Down.IA_Down"))
  ;[1 1 1] Down
  (:`Started`
    (`self.SetButtonHighlighted` (`self.Current Button`))
    (bind _output_get (set `self.Current Button` (+ (`self.Current Button`) (`self.Button Per Row`))))
    (if (not (< _output_get (`KismetArrayLibrary.Array_Length` (`self.Button List`))))
      (set `self.Current Button` (- (`self.Current Button`) (`KismetArrayLibrary.Array_Length` (`self.Button List`)))))
    (`self.SetButtonHighlighted` (`self.Current Button`) true)))

(event `EnhancedInput|/Game/Inputs/Keypad/IA_Up`
  (params (ActionValue :type Boolean) (ElapsedSeconds :type "Float (double-precision)") (TriggeredSeconds :type "Float (double-precision)") (InputAction :type "InputAction Object Reference" :default "/Game/Inputs/Keypad/IA_Up.IA_Up"))
  ;[1 1 1] Up
  (:`Started`
    (`self.SetButtonHighlighted` (`self.Current Button`))
    (bind _output_get (set `self.Current Button` (- (`self.Current Button`) (`self.Button Per Row`))))
    (if (not (>= _output_get 0))
      (set `self.Current Button` (+ (`self.Current Button`) (`KismetArrayLibrary.Array_Length` (`self.Button List`)))))
    (`self.SetButtonHighlighted` (`self.Current Button`) true)))

(event `EnhancedInput|/Game/Inputs/Player/IA_Interact`
  (params (ActionValue :type Boolean) (ElapsedSeconds :type "Float (double-precision)") (TriggeredSeconds :type "Float (double-precision)") (InputAction :type "InputAction Object Reference" :default "/Game/Inputs/Player/IA_Interact.IA_Interact"))
  (:`Started`
    (`KismetSystemLibrary.PrintString` (`KismetStringLibrary.Conv_IntToString` (`self.Current Button`)))
    (bind _returnvalue (`CommonActivatableWidgetContainerBase.BP_AddWidget` (`/Game/UI/WBP_GameUI.PostitHintStack` (`/Game/Blueprint/GM_Basic.GameUI` (`/Game/Blueprint/BP_Player.Game Mode` (`self.Player`)))) "/Game/UI/WBP_Post-Hint.WBP_Post-Hint_C"))
    (`/Game/UI/WBP_Post-Hint.ShowCurrentHint` _returnvalue (`self.Current Button`) self)))

(fn `isInteractable`
  (returns (isInteractable :type Boolean))
  (return (`self.Is Interactable`)))

(fn `UserConstructionScript`
  (set `self.Button List` (`|MakeArray` (`self.BPC_KeypadButton0`) (`self.BPC_KeypadButton1`) null)))