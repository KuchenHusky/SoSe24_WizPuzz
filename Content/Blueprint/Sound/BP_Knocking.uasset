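; Sound Blueprint that endlessly plays paired shouting and knocking sounds, starting one second after BeginPlay.
; PlaySound sets both audio components from parallel arrays using a shared index, which wraps at the knocking array's length.
; A configurable delay then calls PlayAgain to repeat the cycle.
; A zero-time SetTimerByEvent also targets PlayAgain, but the Delay drives the loop.
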(event `self.ReceiveBeginPlay`
  (`KismetSystemLibrary.Delay` 1.0)
  (`self.Play Sound`))

(event `self.ReceiveTick`
  (params (DeltaSeconds :type "Float (single-precision)")))

(event `Play Sound`
  (bind _audio_shouting (`self.Audio_Shouting`))
  (bind _current_sound (`self.Current Sound`))
  (`KismetSystemLibrary.K2_SetTimerDelegate` (delegate `PlayAgain`) :!label _label)
  (`|ExecutionSequence`
    (:`then_0`
      (`AudioComponent.SetSound` _audio_shouting (`|GetArrayItem` (`self.Sounds Shouting`) (`self.Current Sound`)))
      (`AudioComponent.Play` _audio_shouting 0.0))
    (:`then_1`
      (`AudioComponent.SetSound` (`self.Audio_knocking`) (`|GetArrayItem` (`self.Sounds Knocking`) (`self.Current Sound`)))
      (`AudioComponent.Play` (`self.Audio_knocking`) 0.0)
      (bind _result (`/Engine/EditorBlueprintResources/StandardMacros.IncrementInt` _current_sound)
        (:`  `
          (set `self.Current Sound` _result)
          (if (== _current_sound (`KismetArrayLibrary.Array_Length` (`self.Sounds Knocking`)))
            (set `self.Current Sound` 0))
          (`KismetSystemLibrary.Delay` (`self.Delay between Sounds`))
          (`self.PlayAgain`))))))

(event `PlayAgain`
  (goto _label))

(fn `UserConstructionScript`)