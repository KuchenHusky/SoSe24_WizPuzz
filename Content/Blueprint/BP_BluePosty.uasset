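; BP_BluePosty is an interactable, apparently a blue post-it note, that shows the player a hint.
; It caches GM_Basic on BeginPlay and toggles a wavy overlay material on its BPCKeypadButton component as a highlight.
; Interacting pushes a WBP_PostHint widget onto the game UI's post-it hint stack, passing the component's ButtonValue and itself, then hides the gameplay UI stack.
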(event `self.ReceiveBeginPlay`
  (`self.Setup Variables`))

(event `Setup Variables`
  ;[1 1 1] Setup Variables
  (bind _asgm_basic (cast `/Game/Blueprint/GM_Basic` (`GameplayStatics.GetGameMode`)))
  (set `self.GameMode` _asgm_basic))

(event `/Game/Blueprint/Interfaces/BPI_Puzzle.SetHighlight`
  (params (On :type Boolean))
  (`MeshComponent.SetOverlayMaterial` (`self.BPC_KeypadButton`) (select `bool` On :`true` "/Game/Materials/Overlays/M_WaveyTexture.M_WaveyTexture" :!type "MaterialInterface Object Reference")))

(event `/Game/Blueprint/Interfaces/BPI_Puzzle.Interact`
  (params (`Last Possess` :type "Pawn Object Reference"))
  (bind _gameui (`/Game/Blueprint/GM_Basic.GameUI` (`self.GameMode`)))
  (`|ExecutionSequence`
    (:`then_0`
      (bind _returnvalue (`CommonActivatableWidgetContainerBase.BP_AddWidget` (`/Game/UI/WBP_GameUI.PostitHintStack` _gameui) "/Game/UI/WBP_Post-Hint.WBP_Post-Hint_C"))
      (`/Game/UI/WBP_Post-Hint.ShowCurrentHint` _returnvalue (`/Game/Blueprint/Components/BPC_KeypadButton.Button Value` (`self.BPC_KeypadButton`)) self))
    (:`then_1`
      (`Widget.SetVisibility` (`/Game/UI/WBP_GameUI.GameplayStack` _gameui) "Hidden"))))

(fn `isInteractable`
  (returns (isInteractable :type Boolean))
  (return true))

(fn `UserConstructionScript`)