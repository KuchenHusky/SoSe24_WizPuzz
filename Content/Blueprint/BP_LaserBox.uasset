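; BP_LaserBox is an interactable pawn that fires a laser and can be possessed by the player, apparently for a puzzle.
; Interacting hides the game UI and smooth-possesses the box, while highlighting toggles an overlay material on its mesh.
; Each tick, a debug-drawn line trace from the arrow component prints whether the hit component carries the "Empfänger" (receiver) tag.
; Mirror detection and input-mapping logic are unconnected, and possession events are empty.
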(event `self.ReceiveBeginPlay`
  (`self.Setup Variables`))

(event `self.ReceiveTick`
  (params (DeltaSeconds :type "Float (single-precision)"))
  (`self.ShootLaser`))

(event `Setup Variables`
  ;[1 1 1] Setup Variables
  (`|ExecutionSequence`
    (:`then_0`
      (bind _asgm_basic (cast `/Game/Blueprint/GM_Basic` (`GameplayStatics.GetGameMode`)))
      (set `self.Game Mode` _asgm_basic))))

(event `/Game/Blueprint/Interfaces/BPI_Puzzle.SetHighlight`
  (params (On :type Boolean))
  (`MeshComponent.SetOverlayMaterial` (`self.SM_LaserBox`) (select `bool` On :`true` "/Game/Materials/Overlays/MI_WaveTexture.MI_WaveTexture" :!type "MaterialInterface Object Reference")))

(event `/Game/Blueprint/Interfaces/BPI_Puzzle.Interact`
  (params (`Last Possess` :type "Pawn Object Reference"))
  (set `self.Last Possess` `Last Possess`)
  (`Widget.SetVisibility` (`/Game/Blueprint/GM_Basic.GameUI` (`self.Game Mode`)) "Hidden")
  (`/Game/Blueprint/BP_MacroLibary.MySmoothPossess` self 1.0))

(event `self.ReceivePossessed`
  (params (NewController :type "Controller Object Reference"))
  ;[1 1 1] Possesd | Unpossed
)

(event `self.ReceiveUnpossessed`
  (params (OldController :type "Controller Object Reference"))
  ;[1 1 1] Possesd | Unpossed
)

(event `ShootLaser`
  (bind _laser_arrow (`self.Laser Arrow`))
  (bind _returnvalue (`SceneComponent.K2_GetComponentLocation` _laser_arrow))
  (bind _outhit (`KismetSystemLibrary.LineTraceSingle` :`Start` _returnvalue :`End` (+ _returnvalue (* (`SceneComponent.GetForwardVector` _laser_arrow) 5000.0)) :`TraceChannel` "TraceTypeQuery1" :`bTraceComplex` true :`DrawDebugType` "ForOneFrame" :`bIgnoreSelf` false))
  (`KismetSystemLibrary.PrintString` (`KismetStringLibrary.Conv_BoolToString` (`ActorComponent.ComponentHasTag` (`.HitComponent` (`GameplayStatics.BreakHitResult` _outhit)) "Empfänger")) true true (struct :`R` 0.287672 :`G` 1.0 :`A` 1.0)))

(fn `isInteractable`
  (returns (isInteractable :type Boolean))
  (return true))

(fn `UserConstructionScript`)