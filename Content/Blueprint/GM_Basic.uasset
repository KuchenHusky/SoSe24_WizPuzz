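; Basic game mode that sets up the game UI and music and handles player respawn and pausing.
; On BeginPlay it shows WBP_GameUI with an opening post-it widget, locks player movement, caches the PlayerStart transform and plays a delayed music track.
; Death fades the camera out, then spawns and possesses a new BP_Player there.
; PauseGame toggles the pause widget stack and input mode; PlayMusic starts an event instance that EndPlay stops.
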(event `self.ReceiveBeginPlay`
  (`self.SetupUI`) ; Function (SetupUI)
  (`self.Setup Variables`)
  (`self.Setup Music`))

(event `Setup Variables`
  ;[1 1 1] Setup Variables
  (`|ExecutionSequence`
    (:`then_0`
      (bind _returnvalue (`GameplayStatics.GetActorOfClass` "/Script/Engine.PlayerStart"))
      (set `self.Player Spawn Transform` (`self.GetTransform` _returnvalue)))))

(event `Player Died`
  (`PlayerCameraManager.StartCameraFade` :`self` (`GameplayStatics.GetPlayerCameraManager` 0) :`ToAlpha` 1.0 :`Duration` 1.0 :`bHoldWhenFinished` true)
  (`KismetSystemLibrary.Delay` 1.0)
  (`self.PLayer Spawn`))

(event `Player Spawn`
  (bind _player_spawn_transform (`self.Player Spawn Transform`))
  (bind _returnvalue (`|SpawnActorFromClass` "/Game/Blueprint/BP_Player.BP_Player_C" (`KismetMathLibrary.MakeTransform` (.location _player_spawn_transform) (`KismetMathLibrary.MakeRotator` 0.0 0.0 (.yaw (.rotation _player_spawn_transform)))) "Undefined" "MultiplyWithRoot" null null))
  (`Controller.Possess` (`GameplayStatics.GetPlayerController` 0) _returnvalue)
  (`PlayerCameraManager.StartCameraFade` :`self` (`GameplayStatics.GetPlayerCameraManager` 0) :`FromAlpha` 1.0 :`Duration` 1.0 :`bHoldWhenFinished` true))

(event `PauseGame`
  (bind _returnvalue (`GameplayStatics.GetPlayerController` 0))
  (bind _pausestack (`/Game/UI/WBP_GameUI.PauseStack` (`self.GameUI`)))
  (if (not (`GameplayStatics.IsGamePaused`))
    (`CommonActivatableWidgetContainerBase.BP_AddWidget` _pausestack "/Game/UI/WBP_PauseMenuBase.WBP_PauseMenuBase_C")
    (`GameplayStatics.SetGamePaused` true)
    (`WidgetBlueprintLibrary.SetInputMode_UIOnlyEx` _returnvalue null)
    (set `PlayerController.bShowMouseCursor` true _returnvalue)
    (else
      (`CommonActivatableWidgetContainerBase.ClearWidgets` _pausestack)
      (`GameplayStatics.SetGamePaused` false)
      (`WidgetBlueprintLibrary.SetInputMode_GameOnly` _returnvalue)
      (set `PlayerController.bShowMouseCursor` false _returnvalue))))

(event `Play Music`
  (bind _returnvalue (`FMODBlueprintStatics.PlayEvent2D` "/Game/FMOD/Events/Music/InGameMusic.InGameMusic")) ; add In game Music bei Event
  (set `self.Music Track` _returnvalue))

(event `self.ReceiveEndPlay`
  (params (EndPlayReason :type "EEndPlayReason Enum" :default "Destroyed"))
  (`FMODBlueprintStatics.EventInstanceStop` (`self.Music Track`) true))

(event `Setup Music`
  (`KismetSystemLibrary.Delay` 0.5)
  (`GameplayStatics.PlaySound2D` "/Game/Sounds/Music/ES_March_of_the_Gnomes_-_Jon_Bjork.ES_March_of_the_Gnomes_-_Jon_Bjork" 1.0 1.0 0.0 null null))

(fn `SetupUI`
  (bind _returnvalue (`GameplayStatics.GetPlayerController` 0))
  (`|ExecutionSequence`
    (:`then_0`
      (bind _returnvalue_2 (`|CreateWidget` "/Game/UI/WBP_GameUI.WBP_GameUI_C")) ; erstelle das GameUI
      (bind _output_get (set `self.GameUI` _returnvalue_2)) ; WBP_GameUI als Variable
      (`UserWidget.AddToViewport` _output_get 0) ; zeigt es auf den Bildschirm
      (`CommonActivatableWidgetContainerBase.BP_AddWidget` (`/Game/UI/WBP_GameUI.PostitchanStack` _output_get) "/Game/UI/WBP_Post-Begin.WBP_Post-Begin_C") ; aktiviert WBP GameplayUI
      (`WidgetBlueprintLibrary.SetInputMode_UIOnlyEx` _returnvalue null)
      (set `PlayerController.bShowMouseCursor` true _returnvalue)
      (bind _asbp_player (cast `/Game/Blueprint/BP_Player` (`GameplayStatics.GetPlayerCharacter` 0)))
      (set `/Game/Blueprint/BP_Player.Can Move` false _asbp_player))))

(fn `UserConstructionScript`)