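; BP_GoldPlatform is a puzzle platform that plays a Level Sequence once both a gold item and a red bottle have been placed on it.
; Box overlaps identify items by actor tag, set a flag for each and destroy them, with gold also revealing the SMGold mesh.
; TriggerAnimation checks both flags, removes the trigger box, then plays the sequence and removes the mesh if the sequence is valid.
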(event `self.Box.OnComponentBeginOverlap`
  (params (OverlappedComponent :type "PrimitiveComponent Object Reference") (OtherActor :type "Actor Object Reference") (OtherComp :type "PrimitiveComponent Object Reference") (OtherBodyIndex :type Integer) (bFromSweep :type Boolean) (SweepResult :type "HitResult Structure (by ref)"))
  (bind _returnvalue (`self.ActorHasTag` OtherActor "Gold"))
  (if _returnvalue
    (`KismetSystemLibrary.PrintString` (`KismetStringLibrary.Conv_BoolToString` _returnvalue))
    (set `self.Overlapping other Actor` OtherActor)
    (`|ExecutionSequence`
      (:`then_0`
        (`SceneComponent.SetVisibility` (`self.SM_Gold`) true false))
      (:`then_1`
        (`self.K2_DestroyActor` (`self.Overlapping other Actor`))))
    (`self.TriggerAnimation`)
    (set `self.is GoldPlaced` true)
    (elif (`self.ActorHasTag` OtherActor "RedBottle")
      (set `self.Overlapping other Actor` OtherActor)
      (`|ExecutionSequence`
        (:`then_0`
          _)
        (:`then_1`
          (`self.K2_DestroyActor` (`self.Overlapping other Actor`))))
      (`self.TriggerAnimation`)
      (set `self.is RedBottle used` true))))

(event `TriggerAnimation`
  (bind _levelsequence (`self.LevelSequence`))
  (if (and (`self.is GoldPlaced`) (`self.is RedBottle used`))
    (`KismetSystemLibrary.PrintString` "IIAAMMM PLAYYYINNNGGG")
    (`ActorComponent.K2_DestroyComponent` (`self.Box`))
    (`/Engine/EditorBlueprintResources/StandardMacros.IsValid` _levelsequence
      (:`Is Valid`
        (`MovieSceneSequencePlayer.Play` (`LevelSequenceActor.SequencePlayer` _levelsequence))
        (`ActorComponent.K2_DestroyComponent` (`self.SM_Gold`))))))

(fn `UserConstructionScript`)