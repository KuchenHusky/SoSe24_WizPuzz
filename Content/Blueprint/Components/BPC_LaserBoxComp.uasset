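; Laser box component that tracks power state for a puzzle-style laser emitter and supports highlighting.
; On BeginPlay it caches GM_Basic, and highlighting toggles a wave-texture overlay material.
; When received power changes while the box is powered or self-powered, it sends an unpowered message to any valid OtherReceiver.
; It always reports as non-interactable, and its laser-firing and activation calls are disconnected.
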(event `self.ReceiveBeginPlay`
  (`self.Setup Variables`))

(event `self.ReceiveTick`
  (params (DeltaSeconds :type "Float (single-precision)")))

(event `Setup Variables`
  (`|ExecutionSequence`
    (:`then_0`
      (bind _asgm_basic (cast `/Game/Blueprint/GM_Basic` (`GameplayStatics.GetGameMode`)))
      (set `self.Game Mode` _asgm_basic))))

(event `SetHighlight`
  (params (On :type Boolean))
  (`self.SetOverlayMaterial` (select `bool` On :`true` "/Game/Materials/Overlays/MI_WaveTexture.MI_WaveTexture" :!type "MaterialInterface Object Reference")))

(event `/Game/Blueprint/Interfaces/BPI_EnergyReceiver.SetPowered`
  (params (Power :type Boolean))
  (bind _other_receiver (`self.Other Receiver`))
  (if (!= Power (`self.ReceivesPower`))
    (bind _output_get (set `self.ReceivesPower` Power))
    (if (or _output_get (`self.SelfPowered`))
      (`/Engine/EditorBlueprintResources/StandardMacros.IsValid` _other_receiver
        (:`Is Valid`
          (message `/Game/Blueprint/Interfaces/BPI_EnergyReceiver.SetPowered` _other_receiver false))))))

(fn `isInteractable`
  (returns (isInteractable :type Boolean))
  (return false))