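; Possessable laser tower pawn that passes power to whatever energy receiver its beam hits, running when self-powered or powered externally.
; Each tick a forward line trace sets the Niagara beam end and switches BPI_EnergyReceiver targets on or off as the hit changes.
; Interacting blends possession to the tower, whose own input context rotates the cannon or returns to the previous pawn.
; Self-powered towers also fire the trace in the construction script.
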(event `self.ReceiveBeginPlay`
  (`self.Setup Variables`))

(event `/Game/Blueprint/Interfaces/BPI_EnergyReceiver.SetPowered`
  (params (Power :type Boolean))
  (bind _other_receiver (`self.Other Receiver`))
  (if (!= Power (`self.ReceivesPower`))
    (bind _output_get (set `self.ReceivesPower` Power))
    (if (or _output_get (`self.SelfPowered`))
      (`ActorComponent.Activate` (`self.NS_Laser`) false)
      (else
        (`ActorComponent.Deactivate` (`self.NS_Laser`))
        (`/Engine/EditorBlueprintResources/StandardMacros.IsValid` _other_receiver
          (:`Is Valid`
            (message `/Game/Blueprint/Interfaces/BPI_EnergyReceiver.SetPowered` _other_receiver false)))))))

(event `self.ReceiveTick`
  (params (DeltaSeconds :type "Float (single-precision)"))
  (if (or (`self.SelfPowered`) (`self.ReceivesPower`))
    (`self.ShootLaser`)))

(event `/Game/Blueprint/Interfaces/BPI_Puzzle.SetHighlight`
  (params (On :type Boolean))
  (`MeshComponent.SetOverlayMaterial` (`self.SM_LaserTower_LaserBase`) (select `bool` On :`true` "/Game/Materials/Overlays/MI_WaveTexture.MI_WaveTexture" :!type "MaterialInterface Object Reference"))
  (`MeshComponent.SetOverlayMaterial` (`self.SM_LaserTower_LaserCanon`) (select `bool` On :`true` "/Game/Materials/Overlays/MI_WaveTexture.MI_WaveTexture" :!type "MaterialInterface Object Reference")))

(event `/Game/Blueprint/Interfaces/BPI_Puzzle.Interact`
  (params (`Last Possess` :type "Pawn Object Reference"))
  (set `self.Last Possess` `Last Possess`)
  (`Widget.SetVisibility` (`/Game/Blueprint/GM_Basic.GameUI` (`self.Game Mode`)) "Hidden")
  (`/Game/Blueprint/BP_MacroLibary.MySmoothPossess` self 1.0))

(event `Setup Variables`
  ;[1 1 1] Setup Variables
  (`|ExecutionSequence`
    (:`then_0`
      (bind _asgm_basic (cast `/Game/Blueprint/GM_Basic` (`GameplayStatics.GetGameMode`)))
      (set `self.Game Mode` _asgm_basic))))

(event `Exit Tower`
  ;[1 1 1] Exit Tower
  (`self.DisableInput` null)
  (`/Game/Blueprint/BP_MacroLibary.MySmoothPossess` (`self.Last Possess`) 0.5)
  (`self.EnableInput` null))

(event `ShootLaser`
  (bind _other_receiver (`self.Other Receiver`))
  (bind _other_receiver_2 (`self.Other Receiver`))
  (bind _laser_arrow (`self.Laser Arrow`))
  (bind _returnvalue (`SceneComponent.K2_GetComponentLocation` _laser_arrow))
  (bind _returnvalue_2 (+ _returnvalue (* (`SceneComponent.GetForwardVector` _laser_arrow) 5000.0)))
  (bind _outhit (`KismetSystemLibrary.LineTraceSingle` :`Start` _returnvalue :`End` _returnvalue_2 :`TraceChannel` "TraceTypeQuery1" :`DrawDebugType` "ForOneFrame"))
  (bind (_bblockinghit _binitialoverlap _time _distance _location _impactpoint _normal _impactnormal _physmat _hitactor) (`GameplayStatics.BreakHitResult` _outhit))
  (`NiagaraComponent.SetVariableInt` (`self.NS_Laser`) "None" (`KismetMathLibrary.FTrunc` (`KismetMathLibrary.Lerp` _time)))
  (if _bblockinghit
    (`NiagaraComponent.SetVariableVec3` (`self.NS_Laser`) "EndLoc" _location)
    (if (`KismetSystemLibrary.DoesImplementInterface` _hitactor "/Game/Blueprint/Interfaces/BPI_EnergyReceiver.BPI_EnergyReceiver_C")
      (if (!= _other_receiver_2 _hitactor)
        (message `/Game/Blueprint/Interfaces/BPI_EnergyReceiver.SetPowered` _other_receiver_2 false))
      (bind _output_get (set `self.Other Receiver` _hitactor))
      (message `/Game/Blueprint/Interfaces/BPI_EnergyReceiver.SetPowered` _output_get true)
      (else
        (message `/Game/Blueprint/Interfaces/BPI_EnergyReceiver.SetPowered` _other_receiver false :!label _label)
        (set `self.Other Receiver` null)))
    (else
      (`NiagaraComponent.SetVariableVec3` (`self.NS_Laser`) "EndLoc" _returnvalue_2)
      (`/Engine/EditorBlueprintResources/StandardMacros.IsValid` _other_receiver
        (:`Is Valid`
          (goto _label))))))

(event `self.ReceivePossessed`
  (params (NewController :type "Controller Object Reference"))
  ;[1 1 1] Posessed/Unposessed
  (`EnhancedInputSubsystemInterface.AddMappingContext` (pcsubsystem `EnhancedInputLocalPlayerSubsystem` (`GameplayStatics.GetPlayerController` 0)) "/Game/Inputs/LaserTower/IMC_LaserTower.IMC_LaserTower" 0 (struct)))

(event `self.ReceiveUnpossessed`
  (params (OldController :type "Controller Object Reference"))
  ;[1 1 1] Posessed/Unposessed
  (message `EnhancedInputSubsystemInterface.RemoveMappingContext` (pcsubsystem `EnhancedInputLocalPlayerSubsystem` (`GameplayStatics.GetPlayerController` 0)) "/Game/Inputs/LaserTower/IMC_LaserTower.IMC_LaserTower" (struct)))

(event `EnhancedInput|/Game/Inputs/IA_Back`
  (params (ActionValue :type Boolean) (ElapsedSeconds :type "Float (double-precision)") (TriggeredSeconds :type "Float (double-precision)") (InputAction :type "InputAction Object Reference" :default "/Game/Inputs/IA_Back.IA_Back"))
  (:`Started`
    (`self.Exit Tower`)))

(event `EnhancedInput|/Game/Inputs/Player/IA_Look`
  (params (ActionValue :type "Vector2D Structure") (ElapsedSeconds :type "Float (double-precision)") (TriggeredSeconds :type "Float (double-precision)") (InputAction :type "InputAction Object Reference" :default "/Game/Inputs/Player/IA_Look.IA_Look"))
  (:`Triggered`
    (`SceneComponent.K2_AddRelativeRotation` (`self.SM_LaserTower_LaserCanon`) (`KismetMathLibrary.MakeRotator` ActionValue_Y 0.0 ActionValue_X) false false)))

(fn `isInteractable`
  (returns (isInteractable :type Boolean))
  (return true))

(fn `UserConstructionScript`
  (if (`self.SelfPowered`)
    (`self.ShootLaser`)
    (`ActorComponent.SetAutoActivate` (`self.NS_Laser`) true)))