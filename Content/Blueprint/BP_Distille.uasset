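; BP_Distille is a distillery actor that collects ingredients and a bottle, then plays a distilling animation.
; Once the fireplace and oven flags are set, its HitBox destroys overlapping "Bottle" or "Zutat" actors, revealing the bottle mesh or counting ingredients.
; With a bottle and exactly three ingredients, it plays a Level Sequence and removes the bottle mesh shortly after.
; It reports as interactable, but its highlight overlay is disconnected.
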(event `Setup Variables`)

(event `self.HitBox.OnComponentBeginOverlap`
  (params (OverlappedComponent :type "PrimitiveComponent Object Reference") (OtherActor :type "Actor Object Reference") (OtherComp :type "PrimitiveComponent Object Reference") (OtherBodyIndex :type Integer) (bFromSweep :type Boolean) (SweepResult :type "HitResult Structure (by ref)"))
  (bind _returnvalue (`self.ActorHasTag` OtherActor "Bottle"))
  (if (and (`self.is Fireplace done`) (`self.is Ofen done`))
    (if _returnvalue
      (`KismetSystemLibrary.PrintString` (`KismetStringLibrary.Conv_BoolToString` _returnvalue))
      (set `self.Overlapping other Actor` OtherActor)
      (`|ExecutionSequence`
        (:`then_0`
          (`self.K2_DestroyActor` (`self.Overlapping other Actor`))
          (set `self.is Bottle Placed` true)
          (`self.Trigger Animation`))
        (:`then_1`
          (`SceneComponent.SetVisibility` (`self.SM_Bottle`) true false)))
      (elif (`self.ActorHasTag` OtherActor "Zutat")
        (bind _result (`/Engine/EditorBlueprintResources/StandardMacros.IncrementInt` (`self.Zutaten Counter`))
          (:`  `
            (set `self.Zutaten Counter` _result)
            (`|ExecutionSequence`
              (:`then_0`
                (`self.Trigger Animation`))
              (:`then_1`
                (bind _output_get (set `self.Overlapping other Actor` OtherActor))
                (`self.K2_DestroyActor` _output_get)))))))))

(event `Trigger Animation`
  (bind _levelsequence (`self.LevelSequence`))
  (if (and (== (`self.Zutaten Counter`) 3) (`self.is Bottle Placed`))
    (`KismetSystemLibrary.PrintString` "ANIMATION IST RIGGGGGGERDHello")
    (`/Engine/EditorBlueprintResources/StandardMacros.IsValid` _levelsequence
      (:`Is Valid`
        (`MovieSceneSequencePlayer.Play` (`LevelSequenceActor.SequencePlayer` _levelsequence))
        (`KismetSystemLibrary.Delay` 1.05)
        (`ActorComponent.K2_DestroyComponent` (`self.SM_Bottle`))))))

(event `/Game/Blueprint/Interfaces/BPI_Puzzle.SetHighlight`
  (params (On :type Boolean)))

(fn `isInteractable`
  (returns (isInteractable :type Boolean))
  (return true))

(fn `UserConstructionScript`)