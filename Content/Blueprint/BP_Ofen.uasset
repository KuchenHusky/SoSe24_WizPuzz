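; BP_Ofen is an interactable oven puzzle in which the player sets the fire color with a rotating wheel to match a wanted code.
; Interact smooth-possesses the oven, hides the game UI and stops player movement, while possession toggles its input mapping context.
; Directional input drives a timeline turning the wheel 60 degrees per step through six values, each recoloring the Niagara fire.
; Confirming the correct code exits, disables interaction and flags BP_Distille's oven step done.
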(event `self.ReceiveTick`
  (params (DeltaSeconds :type "Float (single-precision)")))

(event `/Game/Blueprint/Interfaces/BPI_Puzzle.Interact`
  (params (`Last Possess` :type "Pawn Object Reference"))
  (bind _output_get (set `self.Last Possess` `Last Possess`))
  (`|ExecutionSequence`
    (:`then_0`
      (`KismetSystemLibrary.PrintString` "Hello")
      (`/Game/Blueprint/BP_MacroLibary.MySmoothPossess` self))
    (:`then_1`
      (bind _asbp_player (cast `/Game/Blueprint/BP_Player` _output_get))
      (bind _output_get_2 (set `self.Player` _asbp_player))
      (set `/Game/Blueprint/BP_Player.Can Move` false _output_get_2)
      (`Widget.SetVisibility` (`/Game/Blueprint/GM_Basic.GameUI` (`/Game/Blueprint/BP_Player.Game Mode` _asbp_player)) "Hidden"))))

(event `ExitOfen`
  (`/Game/Blueprint/BP_MacroLibary.MySmoothPossess` (`self.Last Possess`))
  (`Widget.SetVisibility` (`/Game/Blueprint/GM_Basic.GameUI` (`/Game/Blueprint/BP_Player.Game Mode` (`self.Player`))) "Visible"))

(event `/Game/Blueprint/Interfaces/BPI_Puzzle.SetHighlight`
  (params (On :type Boolean))
  (`MeshComponent.SetOverlayMaterial` (`self.SM_Tube`) (select `bool` On :`true` "/Game/Materials/Overlays/MI_WaveTexture.MI_WaveTexture" :!type "MaterialInterface Object Reference")))

(event `Set Wheel Higlighted`
  (params (Position :type Integer) (Higlight :type Boolean))
  (`/Game/Blueprint/Components/BPC_KeypadButton.SetHighlight` (`|GetArrayItem` (`self.Amount of Wheel`) Position) Higlight))

(event `self.ReceivePossessed`
  (params (NewController :type "Controller Object Reference"))
  (`EnhancedInputSubsystemInterface.AddMappingContext` (pcsubsystem `EnhancedInputLocalPlayerSubsystem` (`GameplayStatics.GetPlayerController` 0)) "/Game/Inputs/Ofen/IMC_Ofen.IMC_Ofen" 0 (struct)))

(event `self.ReceiveUnpossessed`
  (params (OldController :type "Controller Object Reference"))
  (`EnhancedInputSubsystemInterface.RemoveMappingContext` (pcsubsystem `EnhancedInputLocalPlayerSubsystem` (`GameplayStatics.GetPlayerController` 0)) "/Game/Inputs/Ofen/IMC_Ofen.IMC_Ofen" (struct)))

(event `AnimateRotation`
  (bind _current_rotation_roll (`KismetMathLibrary.BreakRotator` (`self.Current Rotation`)))
  (bind _output (`|GetArrayItem` (`self.Amount of Wheel`)))
  (bind _button_value (`/Game/Blueprint/Components/BPC_KeypadButton.Button Value` _output))
  ;[1 1 1] Rotation of Wheel
  (if (`self.Can Controle`)
    (`TimelineComponent.SetPlayRate` (`self.Wheel Rotation`) 2.0)
    (set `self.Current Rotation` (`SceneComponent.RelativeRotation` _output))
    (bind (_direction _alpha) (`Timeline|Wheel Rotation` :!via `PlayFromStart`)
      (:`Update`
        (`SceneComponent.K2_SetRelativeRotation` _output (`KismetMathLibrary.MakeRotator` (`KismetMathLibrary.Lerp` _current_rotation_roll (+ _current_rotation_roll (* 60.0 (`self.Direction`))) _alpha)) false false)
        (set `self.Can Controle` false))
      (:`Finished`
        (set `self.Can Controle` true)
        (set `self.Current Rotation` (`SceneComponent.RelativeRotation` _output))
        (if (== (`self.Direction`) 1.0)
          (bind _result (`/Engine/EditorBlueprintResources/StandardMacros.IncrementInt` _button_value)
            (:`  `
              (bind _output_get (set `/Game/Blueprint/Components/BPC_KeypadButton.Button Value` _result _output))
              (if (> _button_value 6)
                (bind _output_get_2 (set `/Game/Blueprint/Components/BPC_KeypadButton.Button Value` 1 _output))
                (`KismetSystemLibrary.PrintString` (`KismetStringLibrary.Conv_IntToString` _output_get_2) true true (struct :`R` 0.577581 :`G` 0.723055 :`B` 0.130136 :`A` 1.0))
                (`self.ChangeColore` _output_get_2)
                (else
                  (bind _output_get_3 (set `/Game/Blueprint/Components/BPC_KeypadButton.Button Value` _output_get _output))
                  (`KismetSystemLibrary.PrintString` (`KismetStringLibrary.Conv_IntToString` _output_get_3) true true (struct :`R` 0.577581 :`G` 0.723055 :`B` 0.130136 :`A` 1.0))
                  (`self.ChangeColore` _output_get_3)))))
          (else
            (bind _result_2 (`/Engine/EditorBlueprintResources/StandardMacros.DecrementInt` _button_value)
              (:`  `
                (bind _output_get_4 (set `/Game/Blueprint/Components/BPC_KeypadButton.Button Value` _result_2 _output))
                (if (< _button_value 1)
                  (bind _output_get_5 (set `/Game/Blueprint/Components/BPC_KeypadButton.Button Value` 6 _output))
                  (`KismetSystemLibrary.PrintString` (`KismetStringLibrary.Conv_IntToString` _output_get_5) true true (struct :`R` 0.577581 :`G` 0.723055 :`B` 0.130136 :`A` 1.0))
                  (`self.ChangeColore` _output_get_5)
                  (else
                    (bind _output_get_6 (set `/Game/Blueprint/Components/BPC_KeypadButton.Button Value` _output_get_4 _output))
                    (`KismetSystemLibrary.PrintString` (`KismetStringLibrary.Conv_IntToString` _output_get_6) true true (struct :`R` 0.577581 :`G` 0.723055 :`B` 0.130136 :`A` 1.0))
                    (`self.ChangeColore` _output_get_6)))))))))))

(event `ChangeColore`
  (params (ButtonValue :type Integer))
  (bind _currentbuttenvalue (`self.CurrentButtenValue`))
  (bind _currentbuttenvalue_2 (`self.CurrentButtenValue`))
  (bind _currentbuttenvalue_3 (`self.CurrentButtenValue`))
  (bind _currentbuttenvalue_4 (`self.CurrentButtenValue`))
  (bind _currentbuttenvalue_5 (`self.CurrentButtenValue`))
  (bind _returnvalue (`KismetMathLibrary.Conv_IntToDouble` _currentbuttenvalue))
  (bind _returnvalue_2 (`KismetMathLibrary.Conv_IntToDouble` _currentbuttenvalue_3))
  (set `self.CurrentButtenValue` ButtonValue)
  (`|ExecutionSequence`
    (:`then_0`
      (if (== (`self.CurrentButtenValue`) 1)
        (set `self.ColoreValue` (make `LinearColor` 1.0 0.21 0.0 1.0))
        (`NiagaraComponent.SetVariableLinearColor` (`self.NS_Fire`) "Color" (stale _output_get) :!label _label)
        (set `self.CurrentCode` (`KismetStringLibrary.Conv_IntToString` (`self.CurrentButtenValue`)))))
    (:`then_1`
      (if (== _currentbuttenvalue_2 2)
        (bind _output_get (set `self.ColoreValue` (make `LinearColor` (`KismetMathLibrary.Conv_IntToDouble` _currentbuttenvalue_2) 0.0 0.0 1.0)))
        (goto _label)))
    (:`then_2`
      (if (== _currentbuttenvalue_4 3)
        (set `self.ColoreValue` (make `LinearColor` 0.0 (`KismetMathLibrary.Conv_IntToDouble` _currentbuttenvalue_4) 0.0 1.0))
        (goto _label)))
    (:`then_3`
      (if (== _currentbuttenvalue_5 4)
        (set `self.ColoreValue` (make `LinearColor` 0.0 0.0 (`KismetMathLibrary.Conv_IntToDouble` _currentbuttenvalue_5) 1.0))
        (goto _label)))
    (:`then_4`
      (if (== _currentbuttenvalue 5)
        (set `self.ColoreValue` (make `LinearColor` _returnvalue _returnvalue 0.0 1.0))
        (goto _label)))
    (:`then_5`
      (if (== _currentbuttenvalue_3 6)
        (set `self.ColoreValue` (make `LinearColor` _returnvalue_2 0.0 _returnvalue_2 1.0))
        (goto _label)))))

(event `EnhancedInput|/Game/Inputs/IA_Back`
  (params (ActionValue :type Boolean) (ElapsedSeconds :type "Float (double-precision)") (TriggeredSeconds :type "Float (double-precision)") (InputAction :type "InputAction Object Reference" :default "/Game/Inputs/IA_Back.IA_Back"))
  (:`Started`
    (`self.ExitOfen`)))

(event `EnhancedInput|/Game/Inputs/IA_Confirm`
  (params (ActionValue :type Boolean) (ElapsedSeconds :type "Float (double-precision)") (TriggeredSeconds :type "Float (double-precision)") (InputAction :type "InputAction Object Reference" :default "/Game/Inputs/IA_Confirm.IA_Confirm"))
  (:`Started`
    (if (`KismetStringLibrary.EqualEqual_StrStr` (`self.CurrentCode`) (`self.WantedCode`))
      (`KismetSystemLibrary.PrintString` "Richtig" true true (struct :`G` 1.0 :`B` 0.376912 :`A` 1.0))
      (`self.ExitOfen`)
      (set `self.Is Interactable` false)
      (bind _returnvalue (`GameplayStatics.GetActorOfClass` "/Game/Blueprint/BP_Distille.BP_Distille_C"))
      (set `/Game/Blueprint/BP_Distille.is Ofen done` true _returnvalue)
      (`GameplayStatics.PlaySound2D` "/Game/Sounds/MS_Done.MS_Done" 1.0 1.0 0.0 null null))))

(event `EnhancedInput|/Game/Inputs/Keypad/IA_Up`
  (params (ActionValue :type Boolean) (ElapsedSeconds :type "Float (double-precision)") (TriggeredSeconds :type "Float (double-precision)") (InputAction :type "InputAction Object Reference" :default "/Game/Inputs/Keypad/IA_Up.IA_Up"))
  (:`Started`
    (if (`self.Can Controle`)
      (set `self.Direction` 1.0)
      (`self.AnimateRotation` :!label _label))))

(event `EnhancedInput|/Game/Inputs/Keypad/IA_Down`
  (params (ActionValue :type Boolean) (ElapsedSeconds :type "Float (double-precision)") (TriggeredSeconds :type "Float (double-precision)") (InputAction :type "InputAction Object Reference" :default "/Game/Inputs/Keypad/IA_Down.IA_Down"))
  (:`Triggered`
    (if (`self.Can Controle`)
      (set `self.Direction` -1.0)
      (goto _label))))

(event `EnhancedInput|/Game/Inputs/Keypad/IA_Left`
  (params (ActionValue :type Boolean) (ElapsedSeconds :type "Float (double-precision)") (TriggeredSeconds :type "Float (double-precision)") (InputAction :type "InputAction Object Reference" :default "/Game/Inputs/Keypad/IA_Left.IA_Left"))
  (:`Triggered`
    (if (`self.Can Controle`)
      (set `self.Direction` 1.0)
      (`self.AnimateRotation` :!label _label_2))))

(event `EnhancedInput|/Game/Inputs/Keypad/IA_Right`
  (params (ActionValue :type Boolean) (ElapsedSeconds :type "Float (double-precision)") (TriggeredSeconds :type "Float (double-precision)") (InputAction :type "InputAction Object Reference" :default "/Game/Inputs/Keypad/IA_Right.IA_Right"))
  (:`Triggered`
    (if (`self.Can Controle`)
      (set `self.Direction` -1.0)
      (goto _label_2))))

(fn `isInteractable`
  (returns (isInteractable :type Boolean))
  (return (`self.Is Interactable`)))

(fn `UserConstructionScript`
  (set `self.Amount of Wheel` (`|MakeArray` (`self.BPC_KeypadButton`))))