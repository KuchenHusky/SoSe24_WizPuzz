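; BP_Druckplate is an interactable pressure plate that switches laser towers and can trigger a level sequence.
; Interact alternates via FlipFlop: on plays audio, powers the linked Laser tower and plays any LevelSequence; off unpowers every BP_LaserTower_Small in the level.
; Two timelines fade plate and stone emissive up or down, lowering the plate or snapping it back.
; Player overlap begin and end replay only these timelines, without switching lasers.
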(event `/Game/Blueprint/Interfaces/BPI_Puzzle.Interact`
  (params (`Last Possess` :type "Pawn Object Reference"))
  (bind _druckplatte_whiteboxlowpoly_holzplatte_low (`self.Druckplatte_WhiteboxLowPoly_HolzPlatte_low`))
  (bind _druckplatte_whiteboxlowpoly_holzplatte_low_2 (`self.Druckplatte_WhiteboxLowPoly_HolzPlatte_low`))
  (bind _levelsequence (`self.LevelSequence`))
  (`/Engine/EditorBlueprintResources/StandardMacros.FlipFlop`
    (:`A`
      (`AudioComponent.Play` (`self.Audio`) 0.0)
      (`|ExecutionSequence`
        (:`then_0`
          (bind _asbp_laser_tower_small (cast `/Game/Blueprint/BP_LaserTower_Small` (`self.Laser`)))
          (set `/Game/Blueprint/BP_LaserTower_Small.SelfPowered` true _asbp_laser_tower_small)
          (`ActorComponent.Activate` (`/Game/Blueprint/BP_LaserTower_Small.NS_Laser` _asbp_laser_tower_small) false))
        (:`then_1`
          (bind (_direction _alpha) (`Timeline|Timeline` :!label _label)
            (:`Update`
              (`|ExecutionSequence`
                (:`then_0`
                  (bind _returnvalue (`KismetMathLibrary.Lerp` (`self.Base_Emissiv`) (`self.Max_Emissiv`) _alpha))
                  (`MeshComponent.SetScalarParameterValueOnMaterials` _druckplatte_whiteboxlowpoly_holzplatte_low_2 "Emissiv" _returnvalue))
                (:`then_1`
                  (`MeshComponent.SetScalarParameterValueOnMaterials` (`self.Druckplatte_WhiteboxLowPoly_Stein4_low`) "Emissiv" _returnvalue)
                  (`MeshComponent.SetScalarParameterValueOnMaterials` (`self.Druckplatte_WhiteboxLowPoly_Stein3_low`) "Emissiv" _returnvalue)
                  (`MeshComponent.SetScalarParameterValueOnMaterials` (`self.Druckplatte_WhiteboxLowPoly_Stein2_low`) "Emissiv" _returnvalue)
                  (`MeshComponent.SetScalarParameterValueOnMaterials` (`self.Druckplatte_WhiteboxLowPoly_Stein1_low`) "Emissiv" _returnvalue)))
              (`SceneComponent.K2_SetRelativeLocation` _druckplatte_whiteboxlowpoly_holzplatte_low_2 (`KismetMathLibrary.VLerp` (0.0 0.0 0.0) (0.0 0.0 -4.47) _alpha) false false))))
        (:`then_2`
          (`/Engine/EditorBlueprintResources/StandardMacros.IsValid` _levelsequence
            (:`Is Valid`
              (`MovieSceneSequencePlayer.Play` (`LevelSequenceActor.SequencePlayer` _levelsequence)))))))
    (:`B`
      (`|ExecutionSequence`
        (:`then_0`
          (bind (_direction_2 _alpha_2) (`Timeline|Timeline_0` :!via `PlayFromStart` :!label _label_2)
            (:`Update`
              (`|ExecutionSequence`
                (:`then_0`
                  (bind _returnvalue_2 (`KismetMathLibrary.Lerp` (`self.Max_Emissiv`) (`self.Base_Emissiv`) _alpha_2))
                  (`MeshComponent.SetScalarParameterValueOnMaterials` _druckplatte_whiteboxlowpoly_holzplatte_low "Emissiv" _returnvalue_2))
                (:`then_1`
                  (`MeshComponent.SetScalarParameterValueOnMaterials` (`self.Druckplatte_WhiteboxLowPoly_Stein4_low`) "Emissiv" _returnvalue_2)
                  (`MeshComponent.SetScalarParameterValueOnMaterials` (`self.Druckplatte_WhiteboxLowPoly_Stein3_low`) "Emissiv" _returnvalue_2)
                  (`MeshComponent.SetScalarParameterValueOnMaterials` (`self.Druckplatte_WhiteboxLowPoly_Stein2_low`) "Emissiv" _returnvalue_2)
                  (`MeshComponent.SetScalarParameterValueOnMaterials` (`self.Druckplatte_WhiteboxLowPoly_Stein1_low`) "Emissiv" _returnvalue_2)))
              (`SceneComponent.K2_SetRelativeLocation` _druckplatte_whiteboxlowpoly_holzplatte_low (`KismetMathLibrary.VLerp` (0.0 0.0 0.0) (0.0 0.0 0.0) _alpha_2) false false))))
        (:`then_1`
          (bind _outactors (`GameplayStatics.GetAllActorsOfClass` "/Game/Blueprint/BP_LaserTower_Small.BP_LaserTower_Small_C"))
          (for _array_element _outactors
            (bind _output_get (set `self.Array Element` _array_element))
            (set `/Game/Blueprint/BP_LaserTower_Small.SelfPowered` false _output_get)
            (`ActorComponent.Deactivate` (`/Game/Blueprint/BP_LaserTower_Small.NS_Laser` _output_get))))))))

(event `self.BoxCollision.OnComponentBeginOverlap`
  (params (OverlappedComponent :type "PrimitiveComponent Object Reference") (OtherActor :type "Actor Object Reference") (OtherComp :type "PrimitiveComponent Object Reference") (OtherBodyIndex :type Integer) (bFromSweep :type Boolean) (SweepResult :type "HitResult Structure (by ref)"))
  (cast `/Game/Blueprint/BP_Player` OtherActor)
  (goto _label :!via `PlayFromStart`))

(event `self.BoxCollision.OnComponentEndOverlap`
  (params (OverlappedComponent :type "PrimitiveComponent Object Reference") (OtherActor :type "Actor Object Reference") (OtherComp :type "PrimitiveComponent Object Reference") (OtherBodyIndex :type Integer))
  (cast `/Game/Blueprint/BP_Player` OtherActor)
  (goto _label_2 :!via `PlayFromStart`))

(fn `isInteractable`
  (returns (isInteractable :type Boolean))
  (return true))

(fn `UserConstructionScript`)