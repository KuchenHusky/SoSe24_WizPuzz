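; BP_Pickup is a possessable pickup that highlights with an overlay material and, on interact, is picked up by BP_Player if their hand is empty.
; Inspecting possesses the pickup, copies the player camera's transform and moves InspectPivot to the player's inspect point.
; While possessed, its own input mapping context applies: Look rotates the pivot, and Back restores it and repossesses the player.
; Drop detaches the actor and places it at a given transform.
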(event `self.ReceiveBeginPlay`
  (`self.Setup Variables`))

(event `Setup Variables`
  (set `self.OriginalInspectRTransform` (`SceneComponent.GetRelativeTransform` (`self.InspectPivot`))))

(event `/Game/Blueprint/Interfaces/BPI_Puzzle.SetHighlight`
  (params (On :type Boolean))
  (`MeshComponent.SetOverlayMaterial` (`self.SM_NumberCube`) (select `bool` On :`true` "/Game/Materials/Overlays/MI_WaveTexture.MI_WaveTexture" :!type "MaterialInterface Object Reference")))

(event `/Game/Blueprint/Interfaces/BPI_Puzzle.Interact`
  (params (`Last Possess` :type "Pawn Object Reference"))
  (bind _asbp_player (cast `/Game/Blueprint/BP_Player` `Last Possess`))
  (bind _output_get (set `self.Player` _asbp_player))
  (`/Engine/EditorBlueprintResources/StandardMacros.IsValid` (`/Game/Blueprint/BP_Player.Object in Hand` _output_get)
    (:`Is Not Valid`
      (`/Game/Blueprint/BP_Player.Picup Object` (`self.Player`) self))))

(event `Drop`
  (params (NewLocation :type "Vector Structure") (NewRotation :type "Rotator Structure"))
  (`self.K2_DetachFromActor` "KeepRelative")
  (`self.K2_SetActorLocationAndRotation` NewLocation NewRotation))

(event `self.ReceivePossessed`
  (params (NewController :type "Controller Object Reference"))
  (bind _returnvalue (pcsubsystem `EnhancedInputLocalPlayerSubsystem` (`GameplayStatics.GetPlayerController` 0)))
  (`/Engine/EditorBlueprintResources/StandardMacros.IsValid` _returnvalue
    (:`Is Valid`
      (`EnhancedInputSubsystemInterface.AddMappingContext` _returnvalue "/Game/Inputs/Pickup/IMC_Pickup.IMC_Pickup" 0 (struct)))))

(event `self.ReceiveUnpossessed`
  (params (OldController :type "Controller Object Reference"))
  (bind _returnvalue (pcsubsystem `EnhancedInputLocalPlayerSubsystem` (`GameplayStatics.GetPlayerController` 0)))
  (`/Engine/EditorBlueprintResources/StandardMacros.IsValid` _returnvalue
    (:`Is Valid`
      (`EnhancedInputSubsystemInterface.RemoveMappingContext` _returnvalue "/Game/Inputs/Pickup/IMC_Pickup.IMC_Pickup" (struct)))))

(event `Start Inspect`
  (bind _camera (`/Game/Blueprint/BP_Player.Camera` (`self.Player`)))
  (`/Game/Blueprint/BP_MacroLibary.MySmoothPossess` self)
  (`SceneComponent.K2_SetWorldLocationAndRotation` (`self.Camera`) (`SceneComponent.K2_GetComponentLocation` _camera) (`SceneComponent.K2_GetComponentRotation` _camera) false false)
  (`SceneComponent.K2_SetRelativeLocation` (`self.InspectPivot`) (`KismetMathLibrary.InverseTransformLocation` (`self.GetTransform`) (`SceneComponent.K2_GetComponentLocation` (`/Game/Blueprint/BP_Player.InspectLoc` (`self.Player`)))) false false))

(event `Stop Inspect`
  (bind (_originalinspectrtransform_location _originalinspectrtransform_rotation) (`KismetMathLibrary.BreakTransform` (`self.OriginalInspectRTransform`)))
  (`SceneComponent.K2_SetRelativeLocationAndRotation` (`self.InspectPivot`) _originalinspectrtransform_location _originalinspectrtransform_rotation false false)
  (`/Game/Blueprint/BP_MacroLibary.MySmoothPossess` (`self.Player`)))

(event `EnhancedInput|/Game/Inputs/IA_Back`
  (params (ActionValue :type Boolean) (ElapsedSeconds :type "Float (double-precision)") (TriggeredSeconds :type "Float (double-precision)") (InputAction :type "InputAction Object Reference" :default "/Game/Inputs/IA_Back.IA_Back"))
  (:`Started`
    (`self.Stop Inspect`)))

(event `EnhancedInput|/Game/Inputs/Player/IA_Look`
  (params (ActionValue :type "Vector2D Structure") (ElapsedSeconds :type "Float (double-precision)") (TriggeredSeconds :type "Float (double-precision)") (InputAction :type "InputAction Object Reference" :default "/Game/Inputs/Player/IA_Look.IA_Look"))
  (bind _inspectpivot (`self.InspectPivot`))
  (:`Triggered`
    (`SceneComponent.K2_SetRelativeRotation` _inspectpivot (`KismetMathLibrary.ComposeRotators` (`SceneComponent.RelativeRotation` _inspectpivot) (`KismetMathLibrary.MakeRotator` 0.0 (* ActionValue_Y 1.0) (* ActionValue_X 1.0))) false false)))

(fn `isInteractable`
  (returns (isInteractable :type Boolean))
  (return true))

(fn `UserConstructionScript`)