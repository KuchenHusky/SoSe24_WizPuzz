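; Interactable three-wheel combination lock pawn that takes possession from the player, hides the game UI and plays an optional level sequence when solved.
; Its own input mapping context switches the highlighted wheel left/right and rolls it up/down through six values using a 60-degree timeline animation.
; Each roll updates a concatenated code string, which Confirm compares to WantedCode.
; Back or a correct code returns possession and shows the UI.
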(event `/Game/Blueprint/Interfaces/BPI_Puzzle.Interact`
  (params (`Last Possess` :type "Pawn Object Reference"))
  (bind _output_get (set `self.Last Possess` `Last Possess`))
  (`|ExecutionSequence`
    (:`then_0`
      (`KismetSystemLibrary.PrintString` "Hello")
      (`/Game/Blueprint/BP_MacroLibary.MySmoothPossess` self)
      (bind _output_get_2 (set `self.Current Wheel` 0))
      (set `self.Last Interacted Wheel` (`|GetArrayItem` (`self.Amount of Wheel`) (`self.Current Wheel`)))
      (`self.Set Wheel Highlighted` _output_get_2 true))
    (:`then_1`
      (bind _asbp_player (cast `/Game/Blueprint/BP_Player` _output_get))
      (bind _output_get_3 (set `self.Player` _asbp_player))
      (set `/Game/Blueprint/BP_Player.Can Move` false _output_get_3)
      (`Widget.SetVisibility` (`/Game/Blueprint/GM_Basic.GameUI` (`/Game/Blueprint/BP_Player.Game Mode` _asbp_player)) "Hidden"))))

(event `/Game/Blueprint/Interfaces/BPI_Puzzle.SetHighlight`
  (params (On :type Boolean))
  (`MeshComponent.SetOverlayMaterial` (`self.Amount of Wheel`) (select `bool` On :`true` "/Game/Materials/Overlays/MI_WaveTexture.MI_WaveTexture" :!type "MaterialInterface Object Reference")))

(event `Set Wheel Highlighted`
  (params (Position :type Integer) (Highlight :type Boolean))
  (`/Game/Blueprint/Components/BPC_KeypadButton.SetHighlight` (`|GetArrayItem` (`self.Amount of Wheel`) Position) Highlight))

(event `self.ReceivePossessed`
  (params (NewController :type "Controller Object Reference"))
  (set `self.Current Wheel` 0)
  (`EnhancedInputSubsystemInterface.AddMappingContext` (pcsubsystem `EnhancedInputLocalPlayerSubsystem` (`GameplayStatics.GetPlayerController` 0)) "/Game/Inputs/Lock/IMC_Lock.IMC_Lock" 0 (struct)))

(event `self.ReceiveUnpossessed`
  (params (OldController :type "Controller Object Reference"))
  (`EnhancedInputSubsystemInterface.RemoveMappingContext` (pcsubsystem `EnhancedInputLocalPlayerSubsystem` (`GameplayStatics.GetPlayerController` 0)) "/Game/Inputs/Lock/IMC_Lock.IMC_Lock" (struct)))

(event `AnimateRotation`
  (bind _current__rotation_roll (`KismetMathLibrary.BreakRotator` (`self.current  Rotation`)))
  (bind _output (`|GetArrayItem` (`self.Amount of Wheel`) (`self.Current Wheel`)))
  (bind _button_value (`/Game/Blueprint/Components/BPC_KeypadButton.Button Value` _output))
  ;[1 1 1] Roll Animation
  (if (`self.Can Controle`)
    (bind (_direction _alpha) (`Timeline|Wheel Rotation up` :!via `PlayFromStart`)
      (:`Update`
        (`SceneComponent.K2_SetRelativeRotation` _output (`KismetMathLibrary.MakeRotator` (`KismetMathLibrary.Lerp` _current__rotation_roll (+ _current__rotation_roll (* 60.0 (`self.Direction`))) _alpha)) false false)
        (set `self.Can Controle` false))
      (:`Finished`
        (set `self.Can Controle` true)
        (set `self.current  Rotation` (`SceneComponent.RelativeRotation` _output))
        (if (== (`self.Direction`) 1.0)
          (bind _result (`/Engine/EditorBlueprintResources/StandardMacros.IncrementInt` _button_value)
            (:`  `
              (bind _output_get (set `/Game/Blueprint/Components/BPC_KeypadButton.Button Value` _result _output))
              (if (> _button_value 6)
                (bind _output_get_2 (set `/Game/Blueprint/Components/BPC_KeypadButton.Button Value` 1 _output))
                (`KismetSystemLibrary.PrintString` (`KismetStringLibrary.Conv_IntToString` _output_get_2) true true (struct :`R` 0.577581 :`G` 0.723055 :`B` 0.130136 :`A` 1.0))
                (`self.Fill Code Slots` (`self.Current Wheel`) _output_get_2)
                (else
                  (bind _output_get_3 (set `/Game/Blueprint/Components/BPC_KeypadButton.Button Value` _output_get _output))
                  (`KismetSystemLibrary.PrintString` (`KismetStringLibrary.Conv_IntToString` _output_get_3) true true (struct :`R` 0.577581 :`G` 0.723055 :`B` 0.130136 :`A` 1.0))
                  (`self.Fill Code Slots` (`self.Current Wheel`) _output_get_3)))))
          (else
            (bind _result_2 (`/Engine/EditorBlueprintResources/StandardMacros.DecrementInt` _button_value)
              (:`  `
                (bind _output_get_4 (set `/Game/Blueprint/Components/BPC_KeypadButton.Button Value` _result_2 _output))
                (if (< _button_value 1)
                  (bind _output_get_5 (set `/Game/Blueprint/Components/BPC_KeypadButton.Button Value` 6 _output))
                  (`KismetSystemLibrary.PrintString` (`KismetStringLibrary.Conv_IntToString` _output_get_5) true true (struct :`R` 0.577581 :`G` 0.723055 :`B` 0.130136 :`A` 1.0))
                  (`self.Fill Code Slots` (`self.Current Wheel`) _output_get_5)
                  (else
                    (bind _output_get_6 (set `/Game/Blueprint/Components/BPC_KeypadButton.Button Value` _output_get_4 _output))
                    (`KismetSystemLibrary.PrintString` (`KismetStringLibrary.Conv_IntToString` _output_get_6) true true (struct :`R` 0.577581 :`G` 0.723055 :`B` 0.130136 :`A` 1.0))
                    (`self.Fill Code Slots` (`self.Current Wheel`) _output_get_6)))))))))))

(event `Fill Code Slots`
  (params (`Current Wheel` :type Integer) (`Button Value` :type Integer))
  (if (== `Current Wheel` 0)
    (set `self.Code Slot 1` (`KismetStringLibrary.Conv_IntToString` `Button Value`))
    (`self.Set Current Code`)
    (elif (== `Current Wheel` 1)
      (set `self.Code Slot 2` (`KismetStringLibrary.Conv_IntToString` `Button Value`))
      (`self.Set Current Code`)
      (elif (== `Current Wheel` 2)
        (set `self.Code Slot 3` (`KismetStringLibrary.Conv_IntToString` `Button Value`))
        (`self.Set Current Code`)))))

(event `Set Current Code`
  (set `self.Current Code` (`KismetStringLibrary.Concat_StrStr` (`self.Code Slot 1`) (`self.Code Slot 2`) (`self.Code Slot 3`))))

(event `Exit Lock`
  (`/Game/Blueprint/BP_MacroLibary.MySmoothPossess` (`self.Last Possess`))
  (`Widget.SetVisibility` (`/Game/Blueprint/GM_Basic.GameUI` (`/Game/Blueprint/BP_Player.Game Mode` (`self.Player`))) "Visible"))

(event `EnhancedInput|/Game/Inputs/IA_Back`
  (params (ActionValue :type Boolean) (ElapsedSeconds :type "Float (double-precision)") (TriggeredSeconds :type "Float (double-precision)") (InputAction :type "InputAction Object Reference" :default "/Game/Inputs/IA_Back.IA_Back"))
  (:`Triggered`
    (`self.Exit Lock`)))

(event `EnhancedInput|/Game/Inputs/IA_Confirm`
  (params (ActionValue :type Boolean) (ElapsedSeconds :type "Float (double-precision)") (TriggeredSeconds :type "Float (double-precision)") (InputAction :type "InputAction Object Reference" :default "/Game/Inputs/IA_Confirm.IA_Confirm"))
  (bind _level_sequence_to_play (`self.Level Sequence to Play`))
  (:`Started`
    (if (`KismetStringLibrary.EqualEqual_StrStr` (`self.Current Code`) (`self.Wanted Code`))
      (`/Engine/EditorBlueprintResources/StandardMacros.IsValid` _level_sequence_to_play
        (:`Is Valid`
          (`MovieSceneSequencePlayer.Play` (`LevelSequenceActor.SequencePlayer` _level_sequence_to_play)))
        (:`Is Not Valid`
          _))
      (`KismetSystemLibrary.PrintString` "Right" true true (struct :`G` 1.0 :`B` 0.126143 :`A` 1.0))
      (`self.Exit Lock`))))

(event `EnhancedInput|/Game/Inputs/Keypad/IA_Left`
  (params (ActionValue :type Boolean) (ElapsedSeconds :type "Float (double-precision)") (TriggeredSeconds :type "Float (double-precision)") (InputAction :type "InputAction Object Reference" :default "/Game/Inputs/Keypad/IA_Left.IA_Left"))
  ;[1 1 1] Switches between wheels
  (:`Started`
    (if (`self.Can Controle`)
      (`self.Set Wheel Highlighted` (`self.Current Wheel`))
      (bind _result (`/Engine/EditorBlueprintResources/StandardMacros.DecrementInt` (`self.Current Wheel`))
        (:`  `
          (if (not (> _result -1))
            (bind _result_2 (`/Engine/EditorBlueprintResources/StandardMacros.DecrementInt` (`KismetArrayLibrary.Array_Length` (`self.Amount of Wheel`)))
              (:`  `
                (set `self.Current Wheel` _result_2))))
          (`self.Set Wheel Highlighted` (`self.Current Wheel`) true))))))

(event `EnhancedInput|/Game/Inputs/Keypad/IA_Right`
  (params (ActionValue :type Boolean) (ElapsedSeconds :type "Float (double-precision)") (TriggeredSeconds :type "Float (double-precision)") (InputAction :type "InputAction Object Reference" :default "/Game/Inputs/Keypad/IA_Right.IA_Right"))
  ;[1 1 1] Switches between wheels
  (:`Started`
    (if (`self.Can Controle`)
      (`self.Set Wheel Highlighted` (`self.Current Wheel`))
      (bind _result (`/Engine/EditorBlueprintResources/StandardMacros.IncrementInt` (`self.Current Wheel`))
        (:`  `
          (if (not (< _result (`KismetArrayLibrary.Array_Length` (`self.Amount of Wheel`))))
            (set `self.Current Wheel` 0))
          (`self.Set Wheel Highlighted` (`self.Current Wheel`) true))))))

(event `EnhancedInput|/Game/Inputs/Keypad/IA_Up`
  (params (ActionValue :type Boolean) (ElapsedSeconds :type "Float (double-precision)") (TriggeredSeconds :type "Float (double-precision)") (InputAction :type "InputAction Object Reference" :default "/Game/Inputs/Keypad/IA_Up.IA_Up"))
  ;[1 1 1] Rotate Wheel
  (:`Started`
    (if (`self.Can Controle`)
      (set `self.Direction` 1.0)
      (`self.AnimateRotation` :!label _label))))

(event `EnhancedInput|/Game/Inputs/Keypad/IA_Down`
  (params (ActionValue :type Boolean) (ElapsedSeconds :type "Float (double-precision)") (TriggeredSeconds :type "Float (double-precision)") (InputAction :type "InputAction Object Reference" :default "/Game/Inputs/Keypad/IA_Down.IA_Down"))
  ;[1 1 1] Rotate Wheel
  (:`Started`
    (if (`self.Can Controle`)
      (set `self.Direction` -1.0)
      (goto _label))))

(fn `isInteractable`
  (returns (isInteractable :type Boolean))
  (return true))

(fn `UserConstructionScript`
  (set `self.Lock Compones` (`|MakeArray` (`self.BPC_NummernRad | KeypadButton`) (`self.BPC_NummernRad | KeypadButton2`) (`self.BPC_NummernRad | KeypadButton1`) (`self.SM_Lock_ZylinderSchloss`) (`self.SM_Lock_ZylinderSockel`) :!type "StaticMeshComponent Object Reference"))
  (set `self.Amount of Wheel` (`|MakeArray` (`self.BPC_NummernRad | KeypadButton`) (`self.BPC_NummernRad | KeypadButton1`) (`self.BPC_NummernRad | KeypadButton2`))))