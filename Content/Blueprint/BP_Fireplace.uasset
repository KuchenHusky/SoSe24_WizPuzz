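; BP_Fireplace is a fireplace actor that the player fills with wood and lights with flint.
; Overlapping Wood-tagged actors are destroyed, each revealing the next hidden mesh from a construction-script array until the fireplace is full.
; A Flint-tagged actor is then consumed, activating the Niagara fire and setting IsFireplaceDone on the BP_Distille found in the level.
; Debug prints trace the tag checks.
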(event `self.ReceiveBeginPlay`)

(event `self.HitBox.OnComponentBeginOverlap`
  (params (OverlappedComponent :type "PrimitiveComponent Object Reference") (OtherActor :type "Actor Object Reference") (OtherComp :type "PrimitiveComponent Object Reference") (OtherBodyIndex :type Integer) (bFromSweep :type Boolean) (SweepResult :type "HitResult Structure (by ref)"))
  (bind _returnvalue (`self.ActorHasTag` OtherActor "Wood"))
  (bind _returnvalue_2 (`self.ActorHasTag` OtherActor "Flint"))
  (if (not (`self.FirePlace Full`))
    (if _returnvalue
      (set `self.Overlaping Other Actor` OtherActor)
      (`KismetSystemLibrary.PrintString` (`KismetStringLibrary.Conv_BoolToString` _returnvalue) true true (struct :`R` 0.160181 :`G` 1.0 :`B` 0.384205 :`A` 1.0))
      (`|ExecutionSequence`
        (:`then_0`
          (`self.K2_DestroyActor` (`self.Overlaping Other Actor`)))
        (:`then_1`
          (`self.Set Visibility` (`self.FirePlace Full`))))
      (else
        (`KismetSystemLibrary.PrintString` (`KismetStringLibrary.Conv_BoolToString` _returnvalue) true true (struct :`R` 1.0 :`G` 0.123821 :`B` 0.103924 :`A` 1.0))))
    (elif _returnvalue_2
      (`|ExecutionSequence`
        (:`then_0`
          (`self.K2_DestroyActor` OtherActor))
        (:`then_1`
          (set `self.Overlaping Other Actor` OtherActor)
          (`KismetSystemLibrary.PrintString` (`KismetStringLibrary.Conv_BoolToString` _returnvalue_2) true true (struct :`R` 0.160181 :`G` 1.0 :`B` 0.384205 :`A` 1.0))
          (`ActorComponent.Activate` (`self.NS_fire`) false)
          (set `self.Is burnig` true)
          (`self.Cast to Distile`)
          (`ActorComponent.Activate` (`self.NS_fire`) true)))
      (else
        (`KismetSystemLibrary.PrintString` (`KismetStringLibrary.Conv_BoolToString` _returnvalue_2) true true (struct :`R` 1.0 :`G` 0.123821 :`B` 0.103924 :`A` 1.0))))))

(event `Set Visibility`
  (params (`FirePlace Full` :type Boolean))
  (bind _output (`|GetArrayItem` (`self.List of Wood`) (`self.Current Wood`)))
  (if (not `FirePlace Full`)
    (`KismetSystemLibrary.PrintString` (`KismetSystemLibrary.GetDisplayName` _output))
    (`SceneComponent.SetVisibility` _output true false)
    (bind _result (`/Engine/EditorBlueprintResources/StandardMacros.IncrementInt` (`self.Current Wood`))
      (:`  `
        (bind _output_get (set `self.Current Wood` _result))
        (if (== _output_get (`KismetArrayLibrary.Array_Length` (`self.List of Wood`)))
          (set `self.FirePlace Full` true))))))

(event `Cast to Distile`
  (bind _returnvalue (`GameplayStatics.GetActorOfClass` "/Game/Blueprint/BP_Distille.BP_Distille_C"))
  (set `/Game/Blueprint/BP_Distille.is Fireplace done` true _returnvalue))

(fn `UserConstructionScript`
  (set `self.List of Wood` (`|MakeArray` (`self.SM_Wood`) (`self.SM_Wood1`) (`self.SM_Wood2`) (`self.SM_Wood3`))))